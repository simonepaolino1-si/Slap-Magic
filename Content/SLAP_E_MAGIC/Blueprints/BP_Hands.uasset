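; BP_Hands is the slap melee weapon, animated with Paper2D flipbooks.
; ShootWeapon passes a DoOnce gate, plays the slap flipbook, enables HitBox for queries and sends base slap damage to every overlapping BP_EnemyBase.
; After a delay matching the flipbook length, it disables the hit box, restores the idle hands and calls ResetWeapon to reopen the gate.
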(event Custom|ResetWeapon
  (bind _fb_slap (Variables|Default|GetFB_Slap))
  (bind _hitbox (Variables|Default|GetHitBox))
  ;[0.15 0.15 0.15 0.5] Event Shoot (Animazione Schiaffo)
  (Utilities|FlowControl|DoOnce false) ; enters at Reset
)

(event EventShootWeapon
  (bind _fb_slap (Variables|Default|GetFB_Slap))
  (bind _hitbox (Variables|Default|GetHitBox))
  ;[0.15 0.15 0.15 0.5] Event Shoot (Animazione Schiaffo)
  (Utilities|FlowControl|DoOnce false
    (:Completed
      (Sprite|SetFlipbook _fb_slap "/Game/SLAP_E_MAGIC/FlipBook_Mano/FB_Slap.FB_Slap")
      ;[0.15 0.15 0.15 0.5] Collision-Based Melee
      (Collision|SetCollisionEnabled _hitbox "QueryOnly")
      (Development|PrintString "ESCE")
      (for _array_element (Collision|GetOverlappingActors _hitbox "/Game/SLAP_E_MAGIC/Blueprints/Enemy/BP_EnemyBase.BP_EnemyBase_C" :!class /Script/Engine.PrimitiveComponent)
        (Class|BPIHandleDamage|ReceiveDamage(Message) _array_element (Variables|Default|GetbaseSlapDamage)))
      (Utilities|FlowControl|Delay (Class|PaperFlipbookComponent|GetFlipbookLength _fb_slap))
      (Collision|SetCollisionEnabled (Variables|Default|GetHitBox) "NoCollision")
      (Sprite|SetFlipbook (Variables|Default|GetFB_Slap) "/Game/SLAP_E_MAGIC/FlipBook_Mano/FB_Handidle.FB_Handidle")
      (CallFunction|ResetWeapon))))

(fn ConstructionScript
  (|CallParentFunction))
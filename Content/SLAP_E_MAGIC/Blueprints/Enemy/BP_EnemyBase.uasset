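; Base enemy Blueprint with a flipbook visual, health that drops on damage, and destruction shortly after health reaches zero.
; Each Tick updates the health bar widget's percent and rotates it toward the player camera.
; Tick also yaws the actor toward the camera, billboard-style, and derives a walking flag from velocity.
; Flipbook switching is unfinished: its branch leads nowhere, and the timer call has no event bound.
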(event EventBeginPlay)

(event Collision|EventActorBeginOverlap
  (params (OtherActor :type Actor%20Object%20Reference)))

(event EventTick
  (params (DeltaSeconds :type Float%20%28single-precision%29))
  ;[0.15 0.15 0.15 0.5] Logica: HEALTBAR ORIENTATION + DANNO
  (Utilities|FlowControl|Sequence
    (:then_0
      (bind _aswbp_health_bar (Utilities|Casting|CastToWBP_HealthBar (UserInterface|GetWidget (Variables|Default|GetWBP_Health))))
      (Progress|SetPercent (Variables|/Game/SLAP_E_MAGIC/Blueprints/WidgetBlueprint/WBP_HealthBar.WBP_HealthBar_C|GetHP _aswbp_health_bar) (/ (Variables|Default|GetcurrentHealth) (Variables|Default|GetmaxHealth)))
      (Transformation|SetWorldRotation (Variables|Default|GetWBP_Health) (Math|Rotator|FindLookatRotation (Transformation|GetWorldLocation (Variables|Default|GetWBP_Health)) (Transformation|GetWorldLocation (Variables|/Script/Engine.PlayerCameraManager|GetTransformComponent (Game|GetPlayerCameraManager 0)))) false false)
      (if (<= (Variables|Default|GetcurrentHealth) 0.0)
        (Utilities|FlowControl|Delay 0.1)
        (Actor|DestroyActor)))
    (:then_1
      ;[0.15 0.15 0.15 0.5] Logica: ENEMY ORIENTATION
      (Utilities|Time|SetTimerbyEvent 0 0.0)
      (Transformation|SetActorRotation (Math|Rotator|MakeRotator 0.0 0.0 (.Yaw (Math|Rotator|BreakRotator (Math|Rotator|FindLookatRotation (Transformation|GetActorLocation self) (Camera|GetCameraLocation (Game|GetPlayerCameraManager 0)))))))
      (CallFunction|CheckWalkingState)
      (CallFunction|SetCurrentFlipbook))))

(event EventDamage
  (params (damage :type Float%20%28double-precision%29))
  ;[0.15 0.15 0.15 0.5] Evento: RICEVE DANNO
  (Variables|Default|SetcurrentHealth (- (Variables|Default|GetcurrentHealth) damage)))

(fn ConstructionScript)

(fn SetCurrentFlipbook
  (if (Variables|Default|GetisWalking)
    _))

(fn CheckWalkingState
  (if (> (Math|Vector|VectorLength (Variables|/Script/Engine.MovementComponent|GetVelocity (Variables|Character|GetCharacterMovement))) 0.0)
    (Variables|Default|SetisWalking true)
    (else
      (Variables|Default|SetisWalking false))))
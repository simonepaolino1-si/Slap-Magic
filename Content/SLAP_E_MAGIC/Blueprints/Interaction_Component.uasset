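; Interaction component that lets the player focus and use actors tagged "Interactable" at the screen center.
; A count of interactable overlaps starts or stops a looping timer, so sight detection only runs while overlaps exist.
; Detection sphere-traces a short way from the deprojected viewport center, tracks the focused actor and sends it hover and unhover messages.
; The Interact input sends the focused actor an interact message with the component's owner.
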(event Custom|On%20Interactable%20Overlaps
  (params (Overlaps :type Boolean))
  ;[0.15 0.15 0.15 0.5] Overlap_Logic
  (Utilities|FlowControl|Sequence
    (:then_0
      (bind _output_get (Variables|Default|SetOverlapCount (+ (Variables|Default|GetOverlapCount) (select Overlaps 1 -1))))
      (Development|PrintString (Utilities|String|ToString(Integer) _output_get)))
    (:then_1
      (CallFunction|DrawTrace (> (Variables|Default|GetOverlapCount) 0)))))

(event Custom|DrawTrace
  (params (DrawTrace :type Boolean))
  ;[0.15 0.15 0.15 0.5] Draw_Trace_Logic
  (if DrawTrace
    (if (not (Utilities|Time|IsValidTimerHandle (Variables|Default|GetTraceTime)))
      (bind _returnvalue (Utilities|Time|SetTimerbyFunctionName 0 "Detect Sight" 0.1 true))
      (Variables|Default|SetTraceTime _returnvalue))
    (elif (Utilities|Time|IsValidTimerHandle (Variables|Default|GetTraceTime))
      (Utilities|Time|ClearandInvalidateTimerbyHandle (Variables|Default|GetTraceTime))
      (bind _interactableobject (Variables|Default|GetInteractableObject)
        (:then
          (Class|BPInteractableInterface|OnUnHovered(Message) _interactableobject))
        (:else
          _))
      (Variables|Default|SetInteractableObject 0)
      (Variables|Default|SetCan%20Interact false))))

(event Custom|Detect%20Sight
  (bind (_worldlocation _returnvalue) (CallFunction|CalculateTraceStartEnd))
  ;[0.15 0.15 0.15 0.5] Detect Sight
  (bind (_outhit _returnvalue_2) (Collision|SphereTraceByChannel _worldlocation _returnvalue 0.0 "TraceTypeQuery1" false 0 "ForDuration" true "(R=1.000000,G=0.000000,B=0.000000,A=1.000000)" "(R=0.000000,G=1.000000,B=0.000000,A=1.000000)" 0.1))
  (if _returnvalue_2
    (if (Actor|ActorHasTag (.HitActor (Collision|BreakHitResult _outhit)) "Interactable")
      (if (not (== (.HitActor (Collision|BreakHitResult _outhit)) (Variables|Default|GetInteractableObject)))
        (bind _interactableobject (Variables|Default|GetInteractableObject)
          (:then
            (Class|BPInteractableInterface|OnUnHovered(Message) _interactableobject))
          (:else
            _))
        (Variables|Default|SetInteractableObject (.HitActor (Collision|BreakHitResult _outhit)))
        (Variables|Default|SetCan%20Interact true)
        (Class|BPInteractableInterface|OnHovered(Message) (Variables|Default|GetInteractableObject))
        (Development|PrintString "Looking"))
      (else
        (if (Variables|Default|GetCan%20Interact) :!label _label
          (bind _interactableobject_2 (Variables|Default|GetInteractableObject)
            (:then
              (Class|BPInteractableInterface|OnUnHovered(Message) _interactableobject_2))
            (:else
              _))
          (Variables|Default|SetInteractableObject 0)
          (Variables|Default|SetCan%20Interact false)
          (Development|PrintString "Not Looking"))))
    (else
      (goto _label))))

(event Input|EnhancedActionEvents|EnhancedInputActionIA_Interac
  (params (ActionValue :type Boolean) (ElapsedSeconds :type Float%20%28double-precision%29) (TriggeredSeconds :type Float%20%28double-precision%29) (InputAction :type Input%20Action%20Object%20Reference :default "/Game/SLAP_E_MAGIC/Input/Actions/IA_Interac.IA_Interac"))
  ;[0.15 0.15 0.15 0.5] E_Input
  (:Started
    (if (Variables|Default|GetCan%20Interact)
      (Class|BPInteractableInterface|Interact(Message) (Variables|Default|GetInteractableObject) (Components|GetOwner)))))

(fn CalculateTraceStartEnd
  (bind _returnvalue (Game|GetPlayerController 0))
  (bind (_sizex _sizey) (HUD|GetViewportSize _returnvalue))
  (bind _returnvalue_2 (/ _sizex 2))
  (bind _returnvalue_3 (/ _sizey 2))
  (bind _returnvalue_4 (Math|Conversions|ToFloat(Integer) _returnvalue_2))
  (bind _returnvalue_5 (Math|Conversions|ToFloat(Integer) _returnvalue_3))
  (bind (_worldlocation _worlddirection) (Class|PlayerController|DeprojectScreenPositiontoWorld _returnvalue _returnvalue_4 _returnvalue_5))
  (return _worldlocation (+ _worldlocation (* _worlddirection 2.5e+02))))